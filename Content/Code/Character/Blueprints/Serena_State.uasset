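; Serena_State is a character state Blueprint that tracks Serena's health and restarts the level when it runs out.
; Its Health function adds to the health value, clamps it to a normalized range and passes it to the HUD's Bar function.
; If the value Bar returns is zero or below, it reopens the current level by name; otherwise it returns that value.
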(event EventBeginPlay)

(event EventTick
  (params (DeltaSeconds :type Float%20%28single-precision%29)))

(fn ConstructionScript)

(fn Health
  (params (Health_1 :type Float%20%28single-precision%29))
  (bind _output_get (Variables|Default|SetHealth_1 (Math|Float|Clamp(Float) (+ Health_1 (Variables|Default|GetHealth_1)))))
  (bind _result (Default|Bar (Variables|Default|GetHUD%20Ref) _output_get))
  (if (<= _result 0.0)
    (bind _returnvalue (Game|GetCurrentLevelName true))
    (Game|OpenLevel(byName) (Utilities|String|StringToName _returnvalue))
    (else
      (return _result))))